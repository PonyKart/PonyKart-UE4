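; Game mode for the multiplayer gameplay map that spawns players and handles leaving and returning to the lobby.
; It records swapped-in player controllers and respawns a player by replacing their pawn with the given character class at a random PlayerStart.
; Logout asks GameInfoInstance to destroy the session for the exiting GamePlayPC.
; ReturnToLobby, server only, destroys the first player's pawn and server-travels to the Lobby map.
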(event `self.K2_OnSwapPlayerControllers`
  (params (OldPC :type "PlayerController Object Reference") (NewPC :type "PlayerController Object Reference"))
  ;[1 1 1] Keeps track of connected players
  (bind _returnvalue (`KismetArrayLibrary.Array_Add` (`self.AllPlayerControllers`) NewPC))
  (bind _returnvalue_2 (`GameplayStatics.GetPlayerControllerID` NewPC))
  (`KismetSystemLibrary.PrintText` (`|FormatText` "index: {i} Player ControllerIdL {i2}" _returnvalue _returnvalue_2)))

(event `RespawnPlayer`
  (params (PlayerController :type "PlayerController Object Reference") (PlayerCharacter :type "Pawn Class Reference"))
  (bind _returnvalue (`Controller.K2_GetPawn` PlayerController))
  (bind _spawnpoints (`self.SpawnPoints`))
  ;[1 1 1] spawn the player  with the selected character from the GameplayPC
  (bind _outactors (`GameplayStatics.GetAllActorsOfClass` "/Script/Engine.PlayerStart"))
  (set `self.SpawnPoints` _outactors)
  (`/Engine/EditorBlueprintResources/StandardMacros.IsValid` _returnvalue
    (:`Is Valid`
      (`self.K2_DestroyActor` _returnvalue))
    (:`Is Not Valid`
      _))
  (bind _returnvalue_2 (`|SpawnActorFromClass` PlayerCharacter (`self.GetTransform` (`KismetArrayLibrary.Array_Get` _spawnpoints (`KismetMathLibrary.RandomIntegerInRange` 0 (- (`KismetArrayLibrary.Array_Length` _spawnpoints) 1)))) "Undefined" "OverrideRootScale"))
  (`Controller.Possess` PlayerController _returnvalue_2))

(event `self.K2_OnLogout`
  (params (ExitingController :type "Controller Object Reference"))
  ;[1 1 1] EventOnLogout  DestroySessionCaller
  (bind _asgame_play_pc (cast `/Game/Blueprints/GamePlay/GamePlayPC` ExitingController))
  (`/Game/Blueprints/AllLevels/GameInfoInstance.DestroySessionCaller` (cast `/Game/Blueprints/AllLevels/GameInfoInstance` (`GameplayStatics.GetGameInstance`) :!pure true) _asgame_play_pc))

(event `ReturnToLobby`
  (bind _returnvalue (`GameplayStatics.GetPlayerController` 0))
  ;[1 1 1] Return to Lobby. Going to use servertravel seemless
  (if (`KismetSystemLibrary.IsServer`)
    (`self.K2_DestroyActor` (`Controller.K2_GetPawn` _returnvalue))
    (`KismetSystemLibrary.ExecuteConsoleCommand` "servertravel /Game/Maps/Lobby" _returnvalue)))

(fn `UserConstructionScript`)