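; Player-controlled physics hover or kart-style vehicle, driven entirely by forces on CollisionMesh.
; Tick caps speed and runs four corner traces for ground contact and damper values, though the suspension force applied is zero.
; Grounded, it applies lateral friction, speed-scaled downforce, braking, slope-aligned drive and steering torque; airborne, it self-rights.
; Space, labeled drifting, slows global time while held; Escape quits.
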(event `self.ReceiveTick`
  (params (DeltaSeconds :type "Float (single-precision)"))
  (bind _returnvalue (`self.K2_GetActorRotation`))
  (bind _wheelseparationwidth (`self.WheelSeparationWidth`))
  (bind _wheelseparationlength (`self.WheelSeparationLength`))
  (bind _returnvalue_2 (* _wheelseparationlength -1.0))
  (bind _returnvalue_3 (* _wheelseparationwidth -1.0))
  (bind _returnvalue_4 (`KismetMathLibrary.Dot_VectorVector` (`KismetMathLibrary.Normal` (`self.SavedVelocityVector`)) (`SceneComponent.GetForwardVector` (`self.CollisionMesh`))))
  (bind _returnvalue_5 (`KismetMathLibrary.Dot_VectorVector` (`KismetMathLibrary.Normal` (`self.SavedVelocityVector`)) (`SceneComponent.GetRightVector` (`self.CollisionMesh`))))
  ;[1 1 1] Set Values
  (bind _returnvalue_6 (`PrimitiveComponent.GetPhysicsLinearVelocity` (`self.CollisionMesh`) "None"))
  (bind _output_get (set `self.SavedVelocityVector` _returnvalue_6))
  (set `self.SavedVelocityLength` (`KismetMathLibrary.VSize` _output_get))
  (set `self.OnGround` false)
  ;[1 1 1] Velocity Max Speed Control
  (if (> (`self.SavedVelocityLength`) (`self.MaxVelocity`))
    (`PrimitiveComponent.SetPhysicsLinearVelocity` (`self.CollisionMesh`) (* (`KismetMathLibrary.Normal` (`self.SavedVelocityVector`)) (`self.MaxVelocity`)) false "None"))
  (for _index (range 4)
    (bind _returnvalue_7 (+ (`SceneComponent.K2_GetComponentLocation` (`self.CollisionMesh`)) (`KismetMathLibrary.GreaterGreater_VectorRotator` (select `int` _index :`0` (`KismetMathLibrary.MakeVector` _wheelseparationlength _wheelseparationwidth) :`1` (`KismetMathLibrary.MakeVector` _wheelseparationlength _returnvalue_3) :`2` (`KismetMathLibrary.MakeVector` _returnvalue_2 _wheelseparationwidth) :`3` (`KismetMathLibrary.MakeVector` _returnvalue_2 _returnvalue_3)) (`self.K2_GetActorRotation`))))
    ;[1 1 1] LineTraces
    (bind _output_get_2 (set `self.LineTraceStart` _returnvalue_7))
    (bind (_outhit _returnvalue_8) (`KismetSystemLibrary.LineTraceSingle` _output_get_2 (- _returnvalue_7 (* (`SceneComponent.GetUpVector` (`self.CollisionMesh`)) (`self.SuspensionLength`))) "TraceTypeQuery1"))
    ;[1 1 1] Set Values From HitResult
    (if _returnvalue_8
      (set `self.OnGround` true)
      (bind (_bblockinghit _binitialoverlap _time _location _impactpoint _normal _impactnormal) (`GameplayStatics.BreakHitResult` _outhit))
      (set `self.ImpactNormal` _impactnormal)
      (`KismetArrayLibrary.Array_Set` (`self.HitResultLengthPrevious`) _index (`KismetArrayLibrary.Array_Get` (`self.HitResultLenght`) _index))
      (`KismetArrayLibrary.Array_Set` (`self.HitResultLenght`) _index (`KismetMathLibrary.VSize` (- _location (`self.LineTraceStart`))))
      ;[1 1 1] Find Dampener for each suspension point
      (set `self.DamperForce` (* (/ (- (`KismetArrayLibrary.Array_Get` (`self.HitResultLenght`) _index) (`KismetArrayLibrary.Array_Get` (`self.HitResultLengthPrevious`) _index)) (`GameplayStatics.GetGlobalTimeDilation`)) (`self.DamperForceConstant`)))
      ;[1 1 1] Apply Suspension
      (`PrimitiveComponent.AddForceAtLocation` (`self.CollisionMesh`) (0.0 0.0 0.0) (`self.LineTraceStart`) "None")))
  (if (`self.OnGround`)
    (`PrimitiveComponent.SetLinearDamping` (`self.CollisionMesh`) 0.1)
    ;[1 1 1] Lateral Friction and turning
    (`PrimitiveComponent.AddForce` (`self.CollisionMesh`) (* (* (`SceneComponent.GetRightVector` (`self.CollisionMesh`)) (* (* (`KismetMathLibrary.Sqrt` (`KismetMathLibrary.Abs` _returnvalue_5)) (`KismetMathLibrary.SignOfFloat` _returnvalue_5)) (* (`self.SavedVelocityLength`) (`self.LateralFrictionCoefficient `)))) -1.0) "None" true)
    ;[1 1 1] Artificial Grav
    (`PrimitiveComponent.AddForce` (`self.CollisionMesh`) (* (`SceneComponent.GetUpVector` (`self.CollisionMesh`)) (* (`KismetMathLibrary.FClamp` (/ (`self.SavedVelocityLength`) 500.0)) -1500.0)) "None" true)
    ;[1 1 1] Breaking
    (if (`self.Breaking`)
      (`PrimitiveComponent.AddForce` (`self.CollisionMesh`) (* (* (`SceneComponent.GetForwardVector` (`self.CollisionMesh`)) (* (* (`self.SavedVelocityLength`) 2.0) (* (`KismetMathLibrary.Sqrt` (`KismetMathLibrary.Abs` _returnvalue_4)) (`KismetMathLibrary.SignOfFloat` _returnvalue_4)))) -1.0) "None" true))
    ;[1 1 1] Acceleration Control
    (`PrimitiveComponent.AddForce` (`self.CollisionMesh`) (* (* (`KismetMathLibrary.Cross_VectorVector` (`SceneComponent.GetRightVector` (`self.CollisionMesh`)) (`self.ImpactNormal`)) (/ (`self.DriveForce`) (`GameplayStatics.GetGlobalTimeDilation`))) (`self.InputForward`)) "None" true)
    ;[1 1 1] Stearing Control
    (if (>= (`self.SavedVelocityLength`) 100.0)
      (`PrimitiveComponent.AddTorque` (`self.CollisionMesh`) (* (`SceneComponent.GetUpVector` (`self.CollisionMesh`)) (* (* (`KismetMathLibrary.SignOfFloat` (`KismetMathLibrary.Dot_VectorVector` (`self.SavedVelocityVector`) (`SceneComponent.GetForwardVector` (`self.CollisionMesh`)))) (* (`self.InputRight`) (* (`KismetMathLibrary.Lerp` 0.0 1.0 (`KismetMathLibrary.FClamp` (/ (`self.SavedVelocityLength`) 500.0))) (`self.TorqeForce`)))) (`KismetMathLibrary.Sqrt` (`KismetMathLibrary.Abs` (`KismetMathLibrary.Dot_VectorVector` (`KismetMathLibrary.Normal` (`self.SavedVelocityVector`)) (`SceneComponent.GetForwardVector` (`self.CollisionMesh`))))))) "None" true))
    (else
      ;[1 1 1] SelfRighter when in air
      (`PrimitiveComponent.SetLinearDamping` (`self.CollisionMesh`) 0.0)
      (`self.K2_SetActorRotation` (`KismetMathLibrary.RInterpTo` _returnvalue (`KismetMathLibrary.MakeRotFromXZ` (`KismetMathLibrary.Normal` (`KismetMathLibrary.MakeVector` (.x (`KismetMathLibrary.BreakRotIntoAxes` _returnvalue)) (.y (`KismetMathLibrary.BreakRotIntoAxes` _returnvalue)))) (`KismetMathLibrary.MakeVector` 0.0 0.0 1.0)) (`GameplayStatics.GetWorldDeltaSeconds`) 3.0)))))

(event `self.ReceiveBeginPlay`
  (`GameplayStatics.SpawnSoundAttached` "/Game/SoundAndCues/NewSoundCue.NewSoundCue" (`self.CollisionMesh`)))

(event `InputAxis|MoveRight`
  (params (AxisValue :type "Float (single-precision)"))
  (set `self.InputRight` AxisValue))

(event `InputAxis|MoveForward`
  (params (AxisValue :type "Float (single-precision)"))
  (set `self.InputForward` AxisValue))

(event `InputAction|Breaking`
  (params (Key :type "Key Structure" :default "AnyKey"))
  (:`Pressed`
    (set `self.Breaking` true))
  (:`Released`
    (set `self.Breaking` false)))

(event `Key|SpaceBar`
  (params (Key :type "Key Structure" :default "AnyKey"))
  ;[1 1 1] Drifting
  (:`Pressed`
    (`GameplayStatics.SetGlobalTimeDilation` 0.1))
  (:`Released`
    (`GameplayStatics.SetGlobalTimeDilation` 1.0 :!label _label)))

(event `Key|Escape`
  (params (Key :type "Key Structure" :default "AnyKey"))
  (:`Pressed`
    (`KismetSystemLibrary.QuitGame` null "Quit"))
  (:`Released`
    (goto _label)))

(fn `UserConstructionScript`)