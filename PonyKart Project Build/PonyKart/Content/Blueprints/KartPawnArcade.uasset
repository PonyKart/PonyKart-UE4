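; Arcade kart pawn that drives a physics collision mesh with forces and torques instead of simulated wheels.
; Each tick a downward line trace detects ground, feeding spring-damper suspension, lateral friction and self-righting to the surface normal.
; Airborne, it rights toward world up after a short delay; ground and air have separate speed caps.
; Throttle and speed-scaled, direction-aware steering work only on the ground; debug trace and speed readout are active.
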(event `self.ReceiveBeginPlay`
  ;[1 1 1] DEBUG START
  (`PrimitiveComponent.SetPhysicsLinearVelocity` (`self.CollisionMesh`) (0.0 0.0 0.0) true "None")
  (`GameplayStatics.SetGlobalTimeDilation` 1.0)
  (`PrimitiveComponent.SetPhysicsAngularVelocity` (`self.CollisionMesh`) (0.0 0.0 0.0) true "None"))

(event `self.ReceiveTick`
  (params (DeltaSeconds :type "Float (single-precision)"))
  (bind _returnvalue (`KismetMathLibrary.MakeVector` 0.0 0.0 1.0))
  (bind _collisionmesh (`self.CollisionMesh`))
  (bind _maxvelocityonground (`self.MaxVelocityOnGround`))
  (bind _savedvelocity (`self.SavedVelocity`))
  (bind _maxvelocityinair (`self.MaxVelocityInAir`))
  (bind _impactnormal (`self.ImpactNormal`))
  (bind _impactnormal_2 (`self.ImpactNormal`))
  (bind _collisionmesh_2 (`self.CollisionMesh`))
  (bind _collisionmesh_3 (`self.CollisionMesh`))
  (bind _savedvelocity_2 (`self.SavedVelocity`))
  (bind _savedvelocity_3 (`self.SavedVelocity`))
  (bind _returnvalue_2 (`SceneComponent.GetUpVector` (`self.CollisionMesh`)))
  (bind _returnvalue_3 (`SceneComponent.GetUpVector` (`self.CollisionMesh`)))
  (bind _returnvalue_4 (`SceneComponent.K2_GetComponentLocation` _collisionmesh))
  (bind _returnvalue_5 (`SceneComponent.GetRightVector` (`self.CollisionMesh`)))
  (bind _returnvalue_6 (`KismetMathLibrary.Dot_VectorVector` (`KismetMathLibrary.Normal` _savedvelocity_2) _returnvalue_5))
  (`PrimitiveComponent.AddForce` (`self.CollisionMesh`) (0.0 0.0 0.0) "None" true)
  ;[1 1 1] Check if on ground and set values
  (bind (_outhit _returnvalue_7) (`KismetSystemLibrary.LineTraceSingle` :`Start` _returnvalue_4 :`End` (+ _returnvalue_4 (* (`SceneComponent.GetUpVector` _collisionmesh) (* (+ (`self.SuspensionLength`) 5.0) -1.0))) :`TraceChannel` "TraceTypeQuery1" :`DrawDebugType` "ForOneFrame"))
  (set `self.OnGround` _returnvalue_7)
  (bind (_bblockinghit _binitialoverlap _time _location _impactpoint _normal _impactnormal_3) (`GameplayStatics.BreakHitResult` _outhit))
  (set `self.ImpactLocation` _location)
  (set `self.ImpactNormal` _impactnormal_3)
  (bind _returnvalue_8 (`PrimitiveComponent.GetPhysicsLinearVelocity` (`self.CollisionMesh`) "None"))
  (bind _output_get (set `self.SavedVelocity` _returnvalue_8))
  (bind _returnvalue_9 (`KismetMathLibrary.Dot_VectorVector` (`KismetMathLibrary.Normal` _output_get) _impactnormal))
  (set `self.DampenerForce` (* (* _impactnormal (* (* (`KismetMathLibrary.Sqrt` (`KismetMathLibrary.Abs` _returnvalue_9)) (`KismetMathLibrary.SignOfFloat` _returnvalue_9)) (* (`KismetMathLibrary.VSize` _output_get) 8.0))) -1.0))
  ;[1 1 1] SelfRighter
  (if (`self.OnGround`)
    (set `self.RighterDelay` 0.25)
    (`PrimitiveComponent.AddTorque` (`self.CollisionMesh`) (* (`KismetMathLibrary.Cross_VectorVector` _returnvalue_2 _impactnormal_2) (`KismetMathLibrary.Lerp` 500.0 200.0 (/ (+ (`KismetMathLibrary.Dot_VectorVector` _returnvalue_2 _impactnormal_2) 1.0) 2.0))) "None" true)
    ;[1 1 1] Suspension
    (`PrimitiveComponent.AddForce` _collisionmesh_2 (+ (* (`self.ImpactNormal`) (`KismetMathLibrary.Lerp` (`self.SuspensionPower`) 0.0 (/ (`KismetMathLibrary.VSize` (- (`self.ImpactLocation`) (`SceneComponent.K2_GetComponentLocation` (`self.CollisionMesh`)))) (`self.SuspensionLength`)))) (`self.DampenerForce`)) "None" true)
    (`PrimitiveComponent.SetLinearDamping` _collisionmesh_2 0.4)
    ;[1 1 1] Lateral Friction and turning
    (`PrimitiveComponent.AddForce` (`self.CollisionMesh`) (* (* _returnvalue_5 (* (* (`KismetMathLibrary.Sqrt` (`KismetMathLibrary.Abs` _returnvalue_6)) (`KismetMathLibrary.SignOfFloat` _returnvalue_6)) (* (`KismetMathLibrary.VSize` _savedvelocity_2) (`self.LateralFrictionCoefficient `)))) -1.0) "None" true)
    ;[1 1 1] Velocity Max Speed Control
    (if (> (`KismetMathLibrary.VSize` _savedvelocity) _maxvelocityonground)
      (`PrimitiveComponent.SetPhysicsLinearVelocity` (`self.CollisionMesh`) (* (`KismetMathLibrary.Normal` _savedvelocity) _maxvelocityonground) false "None"))
    (`KismetSystemLibrary.PrintText` (`KismetTextLibrary.Conv_IntToText` (`KismetMathLibrary.Round` (/ (`KismetMathLibrary.VSize` (`self.SavedVelocity`)) 100.0))) true true (struct :`G` 0.66 :`B` 1.0 :`A` 1.0) 0.0)
    (else
      (bind _output_get_2 (set `self.RighterDelay` (- (`self.RighterDelay`) (`GameplayStatics.GetWorldDeltaSeconds`))))
      (if (<= _output_get_2 0.0)
        (`PrimitiveComponent.AddTorque` (`self.CollisionMesh`) (* (`KismetMathLibrary.Cross_VectorVector` _returnvalue_3 _returnvalue) (`KismetMathLibrary.Lerp` 200.0 60.0 (/ (+ (`KismetMathLibrary.Dot_VectorVector` _returnvalue_3 _returnvalue) 1.0) 2.0))) "None" true))
      ;[1 1 1] Velocity Max Speed Control
      (if (> (`KismetMathLibrary.VSize` _savedvelocity_3) _maxvelocityinair)
        (`PrimitiveComponent.SetPhysicsLinearVelocity` _collisionmesh_3 (* (`KismetMathLibrary.Normal` _savedvelocity_3) _maxvelocityinair) false "None")
        (`PrimitiveComponent.SetLinearDamping` _collisionmesh_3 0.0))
      (`KismetSystemLibrary.PrintText` (`KismetTextLibrary.Conv_IntToText` (`KismetMathLibrary.Round` (/ (`KismetMathLibrary.VSize` (`self.SavedVelocity`)) 100.0))) true true (struct :`G` 0.66 :`B` 1.0 :`A` 1.0) 0.0))))

(event `InputAxis|MoveForward`
  (params (AxisValue :type "Float (single-precision)"))
  ;[1 1 1] Acceleration Control
  (if (`self.OnGround`)
    (`PrimitiveComponent.AddForce` (`self.CollisionMesh`) (* (* (`KismetMathLibrary.Cross_VectorVector` (`SceneComponent.GetRightVector` (`self.CollisionMesh`)) (`self.ImpactNormal`)) (`self.DriveForce`)) AxisValue) "None" true)))

(event `InputAxis|MoveRight`
  (params (AxisValue :type "Float (single-precision)"))
  ;[1 1 1] Stearing Control
  (if (`self.OnGround`)
    (bind _returnvalue (`PrimitiveComponent.GetPhysicsLinearVelocity` (`self.CollisionMesh`) "None"))
    (`PrimitiveComponent.AddTorque` (`self.CollisionMesh`) (* (`SceneComponent.GetUpVector` (`self.CollisionMesh`)) (* (`KismetMathLibrary.SignOfFloat` (`KismetMathLibrary.Dot_VectorVector` _returnvalue (`SceneComponent.GetForwardVector` (`self.CollisionMesh`)))) (* AxisValue (`KismetMathLibrary.Lerp` 0.0 (`self.TorqeForce`) (`KismetMathLibrary.FClamp` (/ (`KismetMathLibrary.VSize` _returnvalue) 500.0)))))) "None" true)))

(fn `UserConstructionScript`)