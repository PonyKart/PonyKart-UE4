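; A test actor that simulates friction-like damping on a physics-driven Cube component.
; BeginPlay launches the cube along world X at high speed.
; Each Tick applies an opposing acceleration proportional to its current velocity, ignoring mass, so it slows like linear drag.
; A minimum-speed check for that force exists but is disconnected, so damping runs every frame.
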(event `self.ReceiveBeginPlay`
  (`PrimitiveComponent.SetPhysicsLinearVelocity` (`self.Cube`) (10000.0 0.0 0.0) false "None"))

(event `self.ReceiveTick`
  (params (DeltaSeconds :type "Float (single-precision)"))
  (bind _returnvalue (`PrimitiveComponent.GetPhysicsLinearVelocity` (`self.Cube`) "None"))
  (`PrimitiveComponent.AddForce` (`self.Cube`) (* _returnvalue -7.0) "None" true))

(fn `UserConstructionScript`)