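; Physics-driven hover-style kart pawn that simulates suspension, grip, throttle and steering with forces on its collision mesh.
; Each Tick, four corner line traces apply distance-scaled spring forces plus a shared velocity-based damper along the ground normal.
; A center trace gates square-root-scaled lateral friction, a speed cap and input.
; Throttle follows the ground slope; steering torque scales with speed and flips in reverse, with debug prints left in.
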(event `self.ReceiveBeginPlay`
  ;[1 1 1] DEBUG START
  (`PrimitiveComponent.SetPhysicsLinearVelocity` (`self.CollisionMesh`) (0.0 0.0 0.0) true "None")
  (`GameplayStatics.SetGlobalTimeDilation` 1.0)
  (`PrimitiveComponent.SetPhysicsAngularVelocity` (`self.CollisionMesh`) (0.0 0.0 0.0) true "None"))

(event `self.ReceiveTick`
  (params (DeltaSeconds :type "Float (single-precision)"))
  (bind _collisionmesh (`self.CollisionMesh`))
  (bind _suspensioncomponentfrontright (`self.SuspensionComponentFrontRight`))
  (bind _suspensioncomponentbackright (`self.SuspensionComponentBackRight`))
  (bind _suspensioncomponentbackleft (`self.SuspensionComponentBackLeft`))
  (bind _collisionmesh_2 (`self.CollisionMesh`))
  (bind _suspensioncomponentfrontleft (`self.SuspensionComponentFrontLeft`))
  (bind _impactnormal (`self.ImpactNormal`))
  (bind _maxvelocityonground (`self.MaxVelocityOnGround`))
  (bind _returnvalue (`SceneComponent.K2_GetComponentLocation` _suspensioncomponentbackleft))
  (bind _returnvalue_2 (`SceneComponent.K2_GetComponentLocation` _suspensioncomponentfrontright))
  (bind _returnvalue_3 (`SceneComponent.K2_GetComponentLocation` _suspensioncomponentbackright))
  (bind _returnvalue_4 (`SceneComponent.K2_GetComponentLocation` _collisionmesh_2))
  (bind _returnvalue_5 (`SceneComponent.GetRightVector` _collisionmesh))
  (bind _returnvalue_6 (`SceneComponent.K2_GetComponentLocation` _suspensioncomponentfrontleft))
  (bind _returnvalue_7 (* (`self.SuspensionLength`) -1.0))
  ;[1 1 1] Check if on ground and set values
  (bind (_outhit _returnvalue_8) (`KismetSystemLibrary.LineTraceSingle` :`Start` _returnvalue_4 :`End` (+ _returnvalue_4 (* (`SceneComponent.GetUpVector` _collisionmesh_2) (* (+ (`self.SuspensionLength`) 5.0) -1.0))) :`TraceChannel` "TraceTypeQuery1" :`DrawDebugType` "ForOneFrame"))
  (set `self.OnGround` _returnvalue_8)
  (set `self.ImpactNormal` (`.ImpactNormal` (`GameplayStatics.BreakHitResult` _outhit)))
  (bind _returnvalue_9 (`PrimitiveComponent.GetPhysicsLinearVelocity` (`self.CollisionMesh`) "None"))
  (bind _returnvalue_10 (`KismetMathLibrary.Dot_VectorVector` (`KismetMathLibrary.Normal` _returnvalue_9) _impactnormal))
  (bind _returnvalue_11 (* (* _impactnormal (* (* (`KismetMathLibrary.Sqrt` (`KismetMathLibrary.Abs` _returnvalue_10)) (`KismetMathLibrary.SignOfFloat` _returnvalue_10)) (* (`KismetMathLibrary.VSize` _returnvalue_9) 100.0))) -1.0))
  (set `self.DampenerForce` _returnvalue_11)
  (`KismetSystemLibrary.PrintString` (`KismetStringLibrary.Conv_VectorToString` _returnvalue_11) true false (struct :`A` 1.0) 0.01)
  ;[1 1 1] Suspension Line Traces and forces
  (bind (_outhit_2 _returnvalue_12) (`KismetSystemLibrary.LineTraceSingle` :`Start` _returnvalue_6 :`End` (+ _returnvalue_6 (* (`SceneComponent.GetUpVector` _suspensioncomponentfrontleft) _returnvalue_7)) :`TraceChannel` "TraceTypeQuery1" :`DrawDebugType` "ForOneFrame"))
  (bind (_outhit_3 _returnvalue_13) (`KismetSystemLibrary.LineTraceSingle` :`Start` _returnvalue_2 :`End` (+ _returnvalue_2 (* (`SceneComponent.GetUpVector` _suspensioncomponentfrontright) _returnvalue_7)) :`TraceChannel` "TraceTypeQuery1" :`DrawDebugType` "ForOneFrame"))
  (bind (_outhit_4 _returnvalue_14) (`KismetSystemLibrary.LineTraceSingle` :`Start` _returnvalue_3 :`End` (+ _returnvalue_3 (* (`SceneComponent.GetUpVector` _suspensioncomponentbackright) _returnvalue_7)) :`TraceChannel` "TraceTypeQuery1" :`DrawDebugType` "ForOneFrame"))
  (bind (_outhit_5 _returnvalue_15) (`KismetSystemLibrary.LineTraceSingle` :`Start` _returnvalue :`End` (+ _returnvalue (* (`SceneComponent.GetUpVector` _suspensioncomponentbackleft) _returnvalue_7)) :`TraceChannel` "TraceTypeQuery1" :`DrawDebugType` "ForOneFrame"))
  (if _returnvalue_12
    (bind (_bblockinghit _binitialoverlap _time _location _impactpoint _normal _impactnormal_2) (`GameplayStatics.BreakHitResult` _outhit_2))
    (`PrimitiveComponent.AddForceAtLocation` (`self.CollisionMesh`) (+ (* _impactnormal_2 (`KismetMathLibrary.Lerp` (`self.SuspensionPower`) 0.0 (/ (`KismetMathLibrary.VSize` (- _location (`SceneComponent.K2_GetComponentLocation` _suspensioncomponentfrontleft))) (`self.SuspensionLength`)))) (`self.DampenerForce`)) (`SceneComponent.K2_GetComponentLocation` _suspensioncomponentfrontleft) "None"))
  (if _returnvalue_13
    (bind (_bblockinghit_2 _binitialoverlap_2 _time_2 _location_2 _impactpoint_2 _normal_2 _impactnormal_3) (`GameplayStatics.BreakHitResult` _outhit_3))
    (`PrimitiveComponent.AddForceAtLocation` (`self.CollisionMesh`) (+ (* _impactnormal_3 (`KismetMathLibrary.Lerp` (`self.SuspensionPower`) 0.0 (/ (`KismetMathLibrary.VSize` (- _location_2 (`SceneComponent.K2_GetComponentLocation` _suspensioncomponentfrontright))) (`self.SuspensionLength`)))) (`self.DampenerForce`)) (`SceneComponent.K2_GetComponentLocation` _suspensioncomponentfrontright) "None"))
  (if _returnvalue_14
    (bind (_bblockinghit_3 _binitialoverlap_3 _time_3 _location_3 _impactpoint_3 _normal_3 _impactnormal_4) (`GameplayStatics.BreakHitResult` _outhit_4))
    (`PrimitiveComponent.AddForceAtLocation` (`self.CollisionMesh`) (+ (* _impactnormal_4 (`KismetMathLibrary.Lerp` (`self.SuspensionPower`) 0.0 (/ (`KismetMathLibrary.VSize` (- _location_3 (`SceneComponent.K2_GetComponentLocation` _suspensioncomponentbackright))) (`self.SuspensionLength`)))) (`self.DampenerForce`)) (`SceneComponent.K2_GetComponentLocation` _suspensioncomponentbackright) "None"))
  (if _returnvalue_15
    (bind (_bblockinghit_4 _binitialoverlap_4 _time_4 _location_4 _impactpoint_4 _normal_4 _impactnormal_5) (`GameplayStatics.BreakHitResult` _outhit_5))
    (`PrimitiveComponent.AddForceAtLocation` (`self.CollisionMesh`) (+ (* _impactnormal_5 (`KismetMathLibrary.Lerp` (`self.SuspensionPower`) 0.0 (/ (`KismetMathLibrary.VSize` (- _location_4 (`SceneComponent.K2_GetComponentLocation` _suspensioncomponentbackleft))) (`self.SuspensionLength`)))) (`self.DampenerForce`)) (`SceneComponent.K2_GetComponentLocation` _suspensioncomponentbackleft) "None"))
  ;[1 1 1] Lateral Friction and turning
  (if (`self.OnGround`)
    (bind _returnvalue_16 (`PrimitiveComponent.GetPhysicsLinearVelocity` _collisionmesh "None"))
    (bind _returnvalue_17 (`KismetMathLibrary.Dot_VectorVector` (`KismetMathLibrary.Normal` _returnvalue_16) _returnvalue_5))
    (`PrimitiveComponent.AddForce` (`self.CollisionMesh`) (* (* _returnvalue_5 (* (* (`KismetMathLibrary.Sqrt` (`KismetMathLibrary.Abs` _returnvalue_17)) (`KismetMathLibrary.SignOfFloat` _returnvalue_17)) (* (`KismetMathLibrary.VSize` _returnvalue_16) (`self.LateralFrictionCoefficient `)))) -1.0) "None" true))
  ;[1 1 1] Velocity Max Speed Control
  (if (`self.OnGround`)
    (bind _returnvalue_18 (`PrimitiveComponent.GetPhysicsLinearVelocity` (`self.CollisionMesh`) "None"))
    (bind _returnvalue_19 (`KismetMathLibrary.VSize` _returnvalue_18))
    (if (> _returnvalue_19 _maxvelocityonground)
      (`PrimitiveComponent.SetPhysicsLinearVelocity` (`self.CollisionMesh`) (* (`KismetMathLibrary.Normal` _returnvalue_18) _maxvelocityonground) false "None")))
  (`KismetSystemLibrary.PrintString` (`KismetStringLibrary.Conv_IntToString` (`KismetMathLibrary.Round` (/ _returnvalue_19 100.0))) true true (struct :`G` 0.110118 :`B` 1.0 :`A` 1.0) 0.01))

(event `InputAxis|MoveForward`
  (params (AxisValue :type "Float (single-precision)"))
  ;[1 1 1] Acceleration Control
  (if (`self.OnGround`)
    (`PrimitiveComponent.AddForce` (`self.CollisionMesh`) (* (* (`KismetMathLibrary.Cross_VectorVector` (`SceneComponent.GetRightVector` (`self.CollisionMesh`)) (`self.ImpactNormal`)) (`self.DriveForce`)) AxisValue) "None" true)))

(event `InputAxis|MoveRight`
  (params (AxisValue :type "Float (single-precision)"))
  ;[1 1 1] Stearing Control
  (if (`self.OnGround`)
    (bind _returnvalue (`PrimitiveComponent.GetPhysicsLinearVelocity` (`self.CollisionMesh`) "None"))
    (`PrimitiveComponent.AddTorque` (`self.CollisionMesh`) (* (`SceneComponent.GetUpVector` (`self.CollisionMesh`)) (* (`KismetMathLibrary.SignOfFloat` (`KismetMathLibrary.Dot_VectorVector` _returnvalue (`SceneComponent.GetForwardVector` (`self.CollisionMesh`)))) (* AxisValue (`KismetMathLibrary.Lerp` 0.0 (`self.TorqeForce`) (`KismetMathLibrary.FClamp` (/ (`KismetMathLibrary.VSize` _returnvalue) 500.0)))))) "None" true)))

(fn `UserConstructionScript`)