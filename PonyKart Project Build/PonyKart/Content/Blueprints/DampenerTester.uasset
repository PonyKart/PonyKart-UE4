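; DampenerTester is a test Blueprint that pushes its Cube away from nearby surfaces with a hover-style suspension force.
; Each tick, a debug-drawn Visibility line trace runs a short distance along the Cube's local down vector.
; On a hit, it adds force at the Cube's location along the impact normal, fading linearly to zero at full trace length.
; Despite the name, the force has no velocity-based damping term.
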(event `/Game/Blueprints/RaycastTester.ReceiveTick`
  (params (DeltaSeconds :type "Float (single-precision)"))
  (bind _returnvalue (`SceneComponent.K2_GetComponentLocation` (`self.Cube`)))
  (bind (_outhit _returnvalue_2) (`KismetSystemLibrary.LineTraceSingle` :`Start` _returnvalue :`End` (+ _returnvalue (* (`SceneComponent.GetUpVector` (`self.Cube`)) -100.0)) :`TraceChannel` "TraceTypeQuery1" :`DrawDebugType` "ForOneFrame"))
  (if _returnvalue_2
    (bind (_bblockinghit _binitialoverlap _time _location _impactpoint _normal _impactnormal) (`GameplayStatics.BreakHitResult` _outhit))
    (`PrimitiveComponent.AddForceAtLocation` (`self.Cube`) (* _impactnormal (`KismetMathLibrary.Lerp` 90000.0 0.0 (/ (`KismetMathLibrary.VSize` (- _location (`SceneComponent.K2_GetComponentLocation` (`self.Cube`)))) 100.0))) (`SceneComponent.K2_GetComponentLocation` (`self.Cube`)) "None")))

(fn `UserConstructionScript`)